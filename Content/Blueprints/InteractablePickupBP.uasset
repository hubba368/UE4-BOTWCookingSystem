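; Interactable pickup prop that moves via a movement component, damaging enemies it hits.
; The construction script picks a random chalice, stool or pot mesh and sizes and aligns the collision box to it.
; That box drives the movement component, re-assigned every Tick.
; On hit, it damages Enemy-tagged actors and destroys itself, and also breaks on anything not tagged Interactable; a player-holding check is left unwired.
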(event `self.ReceiveBeginPlay`)

(event `self.ReceiveTick`
  (params (DeltaSeconds :type "Float (single-precision)"))
  (`MovementComponent.SetUpdatedComponent` (`self.ObjectMovementComp`) (`self.BoxComp`)))

(event `self.BoxComp.OnComponentHit`
  (params (HitComponent :type "PrimitiveComponent Object Reference") (OtherActor :type "Actor Object Reference") (OtherComp :type "PrimitiveComponent Object Reference") (NormalImpulse :type "Vector Structure") (Hit :type "HitResult Structure (by ref)"))
  (if (!= OtherActor null)
    (if (!= OtherActor "InteractablePickupBP")
      (if (!= OtherComp null)
        (if (`self.ActorHasTag` OtherActor "Enemy")
          (`GameplayStatics.ApplyDamage` OtherActor 50.0 (`GameplayStatics.GetPlayerController` 0) self)
          (`self.K2_DestroyActor`)
          (elif (not (`self.ActorHasTag` OtherActor "Interactable"))
            (`self.K2_DestroyActor`)))))))

(fn `UserConstructionScript`
  (bind _sphere (`self.Sphere`))
  (bind _boxcomp (`self.BoxComp`))
  (`MovementComponent.SetUpdatedComponent` (`self.ObjectMovementComp`) _boxcomp)
  (bind _output_get (set `self.ObjectMeshes` (`|MakeArray` "/Game/Meshes/Chalice.Chalice" "/Game/Meshes/stool.stool" "/Game/Meshes/stool.stool" "/Game/Meshes/pot01.pot01" "/Game/Meshes/pot02.pot02" :!type "StaticMesh Object Reference")))
  (bind _output_get_2 (set `self.TempIndex` (`KismetMathLibrary.RandomIntegerInRange` 0 (- (`KismetArrayLibrary.Array_Length` _output_get) 1))))
  (bind _output (`|GetArrayItem` _output_get _output_get_2))
  (bind _output_get_3 (set `self.TempMat` (`StaticMesh.GetMaterial` _output 0)))
  (`StaticMeshComponent.SetStaticMesh` _sphere _output)
  (`PrimitiveComponent.SetMaterial` _sphere 0 _output_get_3)
  (`BoxComponent.SetBoxExtent` _boxcomp (`.BoxExtent` (`KismetSystemLibrary.GetComponentBounds` _sphere)) true)
  (`SceneComponent.K2_SetWorldRotation` (`self.BoxComp`) (`self.K2_GetActorRotation`) false false))